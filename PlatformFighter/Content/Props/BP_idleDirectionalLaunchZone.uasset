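; Directional launch zone prop that flings the player along the world Y and Z axes after entering its box.
; An overlap from a "Player"-tagged BP_ThirdPersonCharacter waits a configurable delay, zeroes the character's velocity, then applies a mass-dependent impulse.
; Y and Z strengths combine their launch speeds with the matching forward component of two arrow components and the character's Percentage value, leaving X at zero.
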(event OnComponentBeginOverlap(Box)
  (params (OverlappedComponent :type Primitive%20Component%20Object%20Reference) (OtherActor :type Actor%20Object%20Reference) (OtherComp :type Primitive%20Component%20Object%20Reference) (OtherBodyIndex :type Integer) (bFromSweep :type Boolean) (SweepResult :type Hit%20Result%20Structure%20%28by%20ref%29))
  (bind _array_element (Utilities|Array|ForEachLoopwithBreak (Variables|/Script/Engine.Actor|GetTags OtherActor) :!label _label)
    (:LoopBody
      (if (== _array_element "Player")
        (bind _asbp_third_person_character (Utilities|Casting|CastToBP_ThirdPersonCharacter OtherActor))
        (Utilities|FlowControl|Delay (Variables|Default|GetLaunchDelay))
        (Variables|/Script/Engine.MovementComponent|SetVelocity (Variables|/Script/Engine.Character|GetCharacterMovement _asbp_third_person_character) (Math|Vector|MakeVector 0.0 0.0 0.0))
        (Physics|AddImpulse (Variables|/Script/Engine.Character|GetCharacterMovement _asbp_third_person_character) (Math|Vector|MakeVector 0.0 (* (Variables|Default|GetLaunchSpeedY) (.Y (Class|KismetMathLibrary|BreakVector3f (Math|Vector|GetForwardVector (Variables|Default|GetY_Arrow)))) (Variables|/Game/ThirdPerson/Blueprints/BP_ThirdPersonCharacter.BP_ThirdPersonCharacter_C|GetPercentage _asbp_third_person_character)) (* (Variables|Default|GetLaunchSpeedZ) (.Z (Class|KismetMathLibrary|BreakVector3f (Math|Vector|GetForwardVector (Variables|Default|GetZ_Arrow)))) (Variables|/Game/ThirdPerson/Blueprints/BP_ThirdPersonCharacter.BP_ThirdPersonCharacter_C|GetPercentage _asbp_third_person_character))) false)
        (goto _label Break)))))

(event EventBeginPlay)

(event EventTick
  (params (DeltaSeconds :type Float%20%28single-precision%29)))

(fn ConstructionScript)